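; A pickable cube that spins in place and awards coins to the first-person player character when collected.
; Tick adds a fixed roll step to the cube mesh each frame, without delta-time scaling.
; Any overlap with the Box plays an explosion sound, then casts player pawn 0 to FirstPersonCharacter, adds its Coin value to that character's Coins and destroys the actor.
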(event `self.ReceiveTick`
  (params (DeltaSeconds :type "Float (single-precision)"))
  (bind _cube (`self.Cube`))
  (bind (_relativerotation_roll _relativerotation_pitch _relativerotation_yaw) (`KismetMathLibrary.BreakRotator` (`SceneComponent.RelativeRotation` _cube)))
  (`SceneComponent.K2_SetRelativeRotation` _cube (`KismetMathLibrary.MakeRotator` (+ _relativerotation_roll 3.5) _relativerotation_pitch _relativerotation_yaw) false false))

(event `self.Box.OnComponentBeginOverlap`
  (params (OverlappedComponent :type "PrimitiveComponent Object Reference") (OtherActor :type "Actor Object Reference") (OtherComp :type "PrimitiveComponent Object Reference") (OtherBodyIndex :type Integer) (bFromSweep :type Boolean) (SweepResult :type "HitResult Structure (by ref)"))
  (`GameplayStatics.PlaySound2D` "/Game/StarterContent/Audio/Explosion02.Explosion02" 1.0 1.0 0.0 null null)
  (bind _asfirst_person_character (cast `/Game/FirstPersonBP/Blueprints/FirstPersonCharacter` (`GameplayStatics.GetPlayerPawn` 0)))
  (set `/Game/FirstPersonBP/Blueprints/FirstPersonCharacter.coins` (+ (`/Game/FirstPersonBP/Blueprints/FirstPersonCharacter.coins` _asfirst_person_character) (`self.coin`)) _asfirst_person_character)
  (`self.K2_DestroyActor`))

(fn `UserConstructionScript`)